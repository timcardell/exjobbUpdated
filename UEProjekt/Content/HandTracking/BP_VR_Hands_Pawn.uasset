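; VR pawn that turns tracked hand gestures into teleporting and object manipulation.
; A looping timer matches high-confidence hands against gestures read from files, then per-hand handlers dispatch the actions.
; Pointing draws a predicted spline-mesh arc for teleport; the right hand shows a laser, grabs remotely via PhysicsHandle or attaches nearby objects.
; A closed left hand rotates and scales remote grabs from hand positions on Tick; R records a gesture.
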(event Custom|FindGesture
  ;[1 1 1] Read and Recogonize Hand Gestures
  (Utilities|FlowControl|Sequence
    (:then_0
      (switch Utilities|FlowControl|Switch|SwitchonETrackingConfidence (Class|OculusInputFunctionLibrary|GetTrackingConfidence "HandRight") ; Only search for hand gestures when high confindence is attained
        (:High
          (bind _returnvalue (Class|GrabbingGesture|DoesGestureExist (Variables|Default|GetRightHand) (Variables|Default|GetGesturesRightHand)))
          (Default|CallGestureFoundRight _returnvalue))))
    (:then_1
      (switch Utilities|FlowControl|Switch|SwitchonETrackingConfidence (Class|OculusInputFunctionLibrary|GetTrackingConfidence "HandLeft") ; Only search for hand gestures when high confindence is attained
        (:High
          (bind _returnvalue_2 (Class|GrabbingGesture|DoesGestureExist (Variables|Default|GetLeftHand) (Variables|Default|GetGesturesLeftHand)))
          (Default|CallGestureFoundLeft _returnvalue_2))))))

(event Custom|DoThingsWithGestureLeft
  (params (NameOfGest :type String))
  ;[1 1 1] Name of action has to be assigned to
  ; DoesGestureExist in order to work
  ;;[1 1 1] So resizable releases if accedentaly right palm open,unnec to set EVRY time
  (Variables|Default|SetisLeftPalmClosed false)
  (Variables|Default|SetisResizable false)
  (if (not (or (Variables|Default|GetIsPointRight) (Variables|Default|GetIsPalmOpenRight)))
    (Variables|Default|SetIsLeftHand true)
    (Variables|Default|SetIsRightHand false)
    (bind (_ispointleft _ispalmopenleft _ispointright _ispalmopenright _returnvalue) (Class|GrabbingGesture|DoActionorNot NameOfGest (Variables|Default|GetIsLeftHand) (Variables|Default|GetIsRightHand)))
    (Utilities|FlowControl|Sequence
      (:then_0
        (Variables|Default|SetIsPointLeft _ispointleft)
        ;[1 1 1] Release teleport spline if gest changes
        (if (Variables|Default|GetisSplineActive)
          (if (not (Variables|Default|GetIsPointLeft))
            (Development|SetHiddeninGame (Variables|Default|GetmeshSpline) true false)
            (Development|SetHiddeninGame (Variables|Default|GetTeleportation%20ring) true false)
            (Variables|Default|SetisSplineActive false))))
      (:then_1
        (Variables|Default|SetIsPalmOpenLeft _ispalmopenleft))
      (:then_2
        (switch string _returnvalue
          (:Teleport
            (CallFunction|PerformTeleport))
          (:Rock%20On
            (CallFunction|RockSign))
          (:PalmClosed
            (if (not (Variables|Default|GetisLeftPalmClosed))
              (CallFunction|PalmClosedGrab)
              (Variables|Default|SetisLeftPalmClosed true)))
          (:Menu
            (Development|PrintString "Spawn menu"))))
      (:then_3
        (Variables|Default|SetIsPointRight _ispointright))
      (:then_4
        (Variables|Default|SetIsPalmOpenRight _ispalmopenright)))))

(event Custom|DoThingsWithGestureRight
  (params (NameOfGest :type String))
  ;[1 1 1] Name of action has to be assigned to
  ; DoesGestureExist in order to work
  (if (not (Variables|Default|GetIsPointLeft))
    ;;[1 1 1] Remove ray if palm is not open
    (if (Utilities|Enum|Equal(Enum) "PalmOpen" NameOfGest)
      _
      (elif (Variables|Default|GetisRayActive)
        (Development|SetHiddeninGame (Variables|Default|GetObjectTraceSplineMesh) true false)
        (Variables|Default|SetisRayActive false)))
    (Variables|Default|SetIsLeftHand false)
    (Variables|Default|SetIsRightHand true)
    (bind (_ispointleft _ispalmopenleft _ispointright _ispalmopenright _returnvalue) (Class|GrabbingGesture|DoActionorNot NameOfGest (Variables|Default|GetIsLeftHand) (Variables|Default|GetIsRightHand)))
    (Utilities|FlowControl|Sequence
      (:then_0
        (Variables|Default|SetIsPointLeft _ispointleft))
      (:then_1
        (Variables|Default|SetIsPalmOpenLeft _ispalmopenleft))
      (:then_2
        (switch string _returnvalue
          (:Default
            ;[1 1 1] Release object  if grab bool is true but no longer grabbing, is called UNNECESSARY AMOUNT OF TIMES
            (if (and (Utilities|Enum|NotEqual(Enum) _returnvalue "PalmClosed") (Variables|Default|GetgrabbedRightHandBool))
              (Variables|Default|SetgrabbedRightHandBool false)
              (Physics|Components|PhysicsHandle|ReleaseComponent (Variables|Default|GetPhysicsHandle))
              (elif (and (Utilities|Enum|NotEqual(Enum) _returnvalue "PalmClosed") (Variables|Default|GetisGrabbedLocalRight))
                (Variables|Default|SetisGrabbedLocalRight false)
                (Transformation|DetachFromComponent (Variables|Default|GetLocallyGrabbedPbject) "KeepWorld" "KeepWorld" "KeepWorld" true)
                (Physics|SetSimulatePhysics (Variables|Default|GetLocallyGrabbedPbject) true))))
          (:Teleport
            (CallFunction|PerformTeleport))
          (:Grab
            (CallFunction|PerformManipulation)
            (Variables|Default|SetgrabbedRightHandBool true))
          (:Rock%20On
            (CallFunction|RockSign))
          (:PalmOpen
            (CallFunction|TraceforManipulation)
            (if (not (Variables|Default|GetisRayActive))
              (Variables|Default|SetisRayActive true)
              (Development|SetHiddeninGame (Variables|Default|GetObjectTraceSplineMesh) false false)))
          (:PalmClosed
            (CallFunction|LocalManipulationRight)
            (Variables|Default|SetisGrabbedLocalRight true))))
      (:then_3
        (Variables|Default|SetIsPointRight _ispointright)
        ;[1 1 1] Release teleport spline if gest changes
        (if (Variables|Default|GetisSplineActive)
          (if (not (Variables|Default|GetIsPointRight))
            (Development|SetHiddeninGame (Variables|Default|GetmeshSpline) true false)
            (Development|SetHiddeninGame (Variables|Default|GetTeleportation%20ring) true false)
            (Variables|Default|SetisSplineActive false))))
      (:then_4
        (Variables|Default|SetIsPalmOpenRight _ispalmopenright)))))

(event Custom|ChangePhysicsHandleLocation
  ;[1 1 1] Update on tick physics handle location
  (Physics|Components|PhysicsHandle|SetTargetLocation (Variables|Default|GetPhysicsHandle) (Transformation|GetWorldLocation (Variables|Default|GetPhysicsHandlerPlaceHolder)))
  (if (Variables|Default|GetisLeftPalmClosed)
    (Class|PhysicsHandleComponent|SetTargetRotation (Variables|Default|GetPhysicsHandle) (Math|Conversions|RotationFromXVector (- (Transformation|GetWorldLocation (Variables|Default|GetRightHand)) (Transformation|GetWorldLocation (Variables|Default|GetLeftHand)))))))

(event EventBeginPlay
  (Class|HeadMountedDisplayFunctionLibrary|SetTrackingOrigin "Floor")
  (Utilities|FlowControl|Sequence
    (:then_0
      ;[1 1 1] Bind event dispatcher for gestures
      (EventDispatchers|BindEventtoGestureFoundRight (EventDispatchers|CreateEvent :!event Custom|DoThingsWithGestureRight))
      (EventDispatchers|BindEventtoGestureFoundLeft (EventDispatchers|CreateEvent :!event Custom|DoThingsWithGestureLeft)))
    (:then_1
      ;[1 1 1] Read and Recogonize Hand Gestures
      (bind _returnvalue (Class|GrabbingGesture|ReadGestures (Variables|Default|GetDirectory_LeftHand)))
      (Variables|Default|SetGesturesLeftHand _returnvalue)
      (bind _returnvalue_2 (Class|GrabbingGesture|ReadGestures (Variables|Default|GetDirectoryRightHand)))
      (Variables|Default|SetGesturesRightHand _returnvalue_2)
      (bind _returnvalue_3 (Utilities|Time|SetTimerbyEvent (delegate Custom|FindGesture) (Variables|Default|GetUpdateFreq) true)) ; Loops every 0.1 second
      (Variables|Default|SetTimerHandle _returnvalue_3))
    (:then_2
      (Development|SetHiddeninGame (Variables|Default|GetTeleportation%20ring) true false))))

(event EventTick
  (params (DeltaSeconds :type Float%20%28single-precision%29))
  ;[1 1 1] On every tick -> if palm open or point ->  trace
  (Utilities|FlowControl|Sequence
    (:then_0
      (if (or (Variables|Default|GetIsPointRight) (Variables|Default|GetIsPointLeft))
        (CallFunction|TraceforTeleport)))
    (:then_2
      (CallFunction|ChangePhysicsHandleLocation))
    (:then_3
      (CallFunction|SetObjectScale))))

(event Input|KeyboardEvents|R
  (params (Key :type Key%20Structure :default "None"))
  ;[1 1 1] Record Hand Gestures
  (:Pressed
    (Class|GrabbingGesture|RecordGesture (Variables|Default|GetRightHand) (Class|KismetSystemLibrary|GetProjectDirectory) "NEWpalmclosed_right")
    (Development|PrintString "Gesture recorded")))

(fn ConstructionScript)

(fn TraceforTeleport
  (bind _teleportation_ring (Variables|Default|GetTeleportation%20ring))
  (bind _returnvalue (Class|TeleportationFunctionLibrary|FindPointingVector (Variables|Default|GetLeftHand) (Variables|Default|GetRightHand) (Variables|Default|GetIsPointLeft) (Variables|Default|GetIsPointRight)))
  (bind _returnvalue_2 (Class|TeleportationFunctionLibrary|FindUsedHand (Variables|Default|GetLeftHand) (Variables|Default|GetRightHand) (Variables|Default|GetIsPointLeft) (Variables|Default|GetIsPointRight)))
  (bind (_outhit _outpathpositions _outlasttracedestination _returnvalue_3) (Class|GameplayStatics|BlueprintPredictProjectilePathbyObjectType _returnvalue_2 (* (Math|Vector|GetForwardVector _returnvalue) 1e+03) true 1.0 (Variables|Default|GetObject%20Types) false 0 "None"))
  (Utilities|FlowControl|Sequence
    (:then_0
      (if _returnvalue_3
        (Utilities|FlowControl|Sequence
          (:then_0
            (bind _output_get (Variables|Default|SetTeleporting%20Location (.ImpactPoint (Collision|BreakHitResult _outhit))))
            (Transformation|SetWorldLocation _teleportation_ring _output_get false false)
            (Development|SetHiddeninGame _teleportation_ring false false))
          (:then_1
            (CallFunction|CreateTeleportSplineArc)))
        (else
          (Development|SetHiddeninGame (Variables|Default|GetTeleportation%20ring) true false))))
    (:then_1
      (Variables|Default|SetOut%20Path%20Positions _outpathpositions))))

(fn PerformTeleport
  (Transformation|SetWorldLocation (Variables|Default|GetDefaultSceneRoot) (Variables|Default|GetTeleporting%20Location) false false)
  (Development|SetHiddeninGame (Variables|Default|GetTeleportation%20ring) true false)
  (Development|SetHiddeninGame (Variables|Default|GetmeshSpline) true false))

(fn TraceforManipulation
  (bind _spherestart (Variables|Default|GetSphereStart))
  (bind _objecttracespline (Variables|Default|GetObjectTraceSpline))
  (bind _returnvalue (Transformation|GetWorldLocation _spherestart))
  ;[1 1 1] Object interaction lsaer pointer and highlight object
  (bind _outhit (Collision|LineTraceByChannel (Transformation|GetWorldLocation (Variables|Default|GetSphereStart)) (+ (* (- (Transformation|GetWorldLocation (Variables|Default|GetSphereEnd)) _returnvalue) 2e+03) _returnvalue) "TraceTypeQuery1" false 0 "None"))
  (Utilities|FlowControl|Sequence
    (:then_0
      (if (.bBlockingHit (Collision|BreakHitResult _outhit))
        (Spline|SetLocationatSplinePoint _objecttracespline 1 (.Location (Collision|BreakHitResult _outhit)) "World" true)
        (else
          (Spline|SetLocationatSplinePoint _objecttracespline 1 (Spline|GetLocationatSplinePoint _objecttracespline 0 "World") "World" true)))
      (CallFunction|UpdateSplineMesh))))

(fn PerformManipulation
  (bind _spherestart (Variables|Default|GetSphereStart))
  (bind _returnvalue (Transformation|GetWorldLocation _spherestart))
  (bind (_outhit _returnvalue_2) (Collision|LineTraceForObjects (Transformation|GetWorldLocation (Variables|Default|GetSphereStart)) (+ (* (- (Transformation|GetWorldLocation (Variables|Default|GetSphereEnd)) _returnvalue) 2e+03) _returnvalue) (Utilities|Array|MakeArray (Variables|Default|GetgrabbableObjects)) false 0 "None"))
  (if _returnvalue_2
    (Utilities|FlowControl|Sequence
      (:then_0
        (Transformation|SetWorldLocation (Variables|Default|GetPhysicsHandlerPlaceHolder) (.Location (Collision|BreakHitResult _outhit)) false false))
      (:then_1
        (Variables|Default|SetHitComponentForGrab (.HitComponent (Collision|BreakHitResult _outhit)))
        (Variables|Default|SetGrabLocation (.Location (Collision|BreakHitResult _outhit)))
        (Physics|Components|PhysicsHandle|GrabComponentatLocationwithRotation (Variables|Default|GetPhysicsHandle) (Variables|Default|GetHitComponentForGrab) "None" (Variables|Default|GetGrabLocation) "0, 0, 0")
        (Development|PrintString (Utilities|GetDisplayName (Variables|Default|GetHitComponentForGrab)))))))

(fn RockSign
  (Development|PrintString "Rock On"))

(fn CreateTeleportSplineArc
  (bind _meshspline (Variables|Default|GetmeshSpline))
  (bind _meshspline_2 (Variables|Default|GetmeshSpline))
  (bind _teleportspline (Variables|Default|GetTeleportSpline))
  (bind _teleportspline_2 (Variables|Default|GetTeleportSpline))
  (bind _out_path_positions (Variables|Default|GetOut%20Path%20Positions))
  (Spline|SetSplinePoints _teleportspline_2 _out_path_positions "World" true)
  (for _index (range 1 (Spline|GetNumberOfSplinePoints _teleportspline_2))
    (if (!= (Utilities|Array|Length _out_path_positions) (Utilities|Array|Length (Variables|Default|GetmeshSpline)))
      (for _array_element _meshspline
        (Components|DestroyComponent _array_element))
      (Utilities|Array|Clear _meshspline)
      (for _index_2 (range 1 (Spline|GetNumberOfSplinePoints (Variables|Default|GetTeleportSpline)))
        (bind _returnvalue (AddComponent|AddSplineMeshComponent true))
        (Utilities|Array|Add _meshspline_2 _returnvalue)))
    (SplineMesh|SetStartandEnd (Utilities|Array|Get(acopy) _meshspline_2 (- _index 1)) (.Location (Spline|GetLocationandTangentatSplinePoint _teleportspline (- _index 1) "World")) (.Tangent (Spline|GetLocationandTangentatSplinePoint _teleportspline (- _index 1) "World")) (.Location (Spline|GetLocationandTangentatSplinePoint _teleportspline _index "World")) (.Tangent (Spline|GetLocationandTangentatSplinePoint _teleportspline _index "World")) true :!class /Script/Engine.SplineMeshComponent)
    (Variables|Default|SetisSplineActive true)))

(fn PalmClosedGrab
  (if (Variables|Default|GetgrabbedRightHandBool)
    (Variables|Default|SetisResizable true)
    (bind _returnvalue (Class|TestFunctionLibrary|SetInitialDistance (Variables|Default|GetLeftHand) (Variables|Default|GetRightHand)))
    (Variables|Default|SetInitialHandDistanceForScale _returnvalue)
    (Variables|Default|SetInitialObjectScale (Transformation|GetWorldScale (Variables|Default|GetHitComponentForGrab)))
    (else
      (Variables|Default|SetisResizable false))))

(fn SetObjectScale
  (if (Variables|Default|GetisResizable)
    (bind _returnvalue (Class|TestFunctionLibrary|SetInitialDistance (Variables|Default|GetLeftHand) (Variables|Default|GetRightHand)))
    (Transformation|SetWorldScale3D (Variables|Default|GetHitComponentForGrab) (* (Variables|Default|GetInitialObjectScale) (/ _returnvalue (Variables|Default|GetInitialHandDistanceForScale))))))

(fn UpdateSplineMesh
  (bind _objecttracespline (Variables|Default|GetObjectTraceSpline))
  (SplineMesh|SetStartandEnd (Variables|Default|GetObjectTraceSplineMesh) (Spline|GetLocationatSplinePoint _objecttracespline 0 "Local") (Spline|GetTangentatSplinePoint _objecttracespline 0 "Local") (Spline|GetLocationatSplinePoint _objecttracespline 1 "Local") (Spline|GetTangentatSplinePoint _objecttracespline 1 "Local") true :!class /Script/Engine.SplineMeshComponent))

(fn LocalManipulationRight
  (bind _outcomponents (Class|KismetSystemLibrary|ComponentOverlapComponents (Variables|Default|GetGrabSphere) (Transformation|GetWorldTransform (Variables|Default|GetRightHand)) (Utilities|Array|MakeArray "ObjectTypeQuery7")))
  (for _array_element _outcomponents
    (bind _output_get (Variables|Default|SetLocallyGrabbedPbject _array_element))
    (Transformation|AttachComponentToComponent _output_get (Variables|Default|GetRight) "None" "KeepWorld" "KeepWorld" "KeepWorld" true)))